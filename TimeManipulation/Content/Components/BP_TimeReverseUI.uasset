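; Component that toggles a wheel selection UI (WI_WheelSelection) with the E key, pausing the game while it is shown.
; It counts overlapping interaction areas through the player's InteractorController events, so interactables take priority and E only toggles the wheel when none overlap.
; A FlipFlop alternates between creating and showing the widget, and triggering its selected button, removing it and restoring game-only input.
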(event Custom|Entered%20interaction
  (params (Interaction%20Actor :type Actor%20Object%20Reference) (Interaction%20Component :type Interaction%20Component%20Object%20Reference))
  ;[0.059 0.4375 0] Tracks how many interactions the player is overlapping
  (Math|Integer|IncrementInt (Variables|Default|GetOverlappingInteractions)))

(event Custom|Leave%20interaction
  (params (Interaction%20Actor :type Actor%20Object%20Reference) (Interaction%20Component :type Interaction%20Component%20Object%20Reference))
  ;[0.059 0.4375 0] Tracks how many interactions the player is overlapping
  (Math|Integer|DecrementInt (Variables|Default|GetOverlappingInteractions)))

(event EventBeginPlay
  (bind _returnvalue (Game|GetPlayerCharacter 0))
  (bind _returnvalue_2 (Actor|GetComponentbyClass _returnvalue "/GAD2010Interaction/InteractorController.InteractorController_C"))
  ;[0.059 0.4375 0] Tracks how many interactions the player is overlapping
  (Utilities|IsValid _returnvalue_2
    (:Is%20Valid
      (EventDispatchers|BindEventtoOnInteractionAreaExit _returnvalue_2 (delegate Custom|Leave%20interaction))
      (EventDispatchers|BindEventtoOnInteractionAreaEnter _returnvalue_2 (delegate Custom|Entered%20interaction)))))

(event Input|KeyboardEvents|E
  (params (Key :type Key%20Structure :default "None"))
  (bind _returnvalue (Game|GetPlayerController 0))
  ;[0.059 0.4375 0] Checks if the player is overlapping with a interactable. If so. the interactable has priority over the UI and UI won't open
  (:Pressed
    (if (== (Variables|Default|GetOverlappingInteractions) 0)
      ;[0.059 0.4375 0] Flips between opening and closing UI
      (Utilities|FlowControl|FlipFlop
        (:A
          ;[0.059 0.4375 0] Checks if UI exists already
          (Utilities|IsValid (Variables|Default|GetUIWidget)
            (:Is%20Valid
              _)
            (:Is%20Not%20Valid
              ;[0.059 0.4375 0] Opens the UI on screen and pauses the game
              (bind _returnvalue_2 (UserInterface|CreateWidget "/TimeManipulation/UI/WI_WheelSelection.WI_WheelSelection_C" _returnvalue))
              (Variables|Default|SetUIWidget _returnvalue_2)))
          (UserInterface|Viewport|AddtoViewport (Variables|Default|GetUIWidget) 0)
          (Input|SetInputModeGameandUI _returnvalue (Variables|Default|GetUIWidget) "DoNotLock" true false)
          (Game|SetGamePaused true))
        (:B
          ;[0.059 0.4375 0] Removes UI from screen, unpauses game.
          (Default|TriggerSelectedButton (Variables|Default|GetUIWidget))
          (Widget|RemovefromParent (Variables|Default|GetUIWidget))
          (Input|SetInputModeGameOnly (Game|GetPlayerController 0) false)
          (Game|SetGamePaused false)
          (Variables|Default|SetUIWidget 0))))))