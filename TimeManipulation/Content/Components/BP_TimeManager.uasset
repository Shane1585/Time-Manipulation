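; Time manager that starts and stops rewinding on BP_TimeReverse components of actors with a given tag, and drives the screen rewind effect.
; Shortly after BeginPlay it binds to the start and stop events of those components on "Time"-tagged actors, keeping a clamped count of rewinding actors.
; While the count is above zero, it applies an effect material to an unbound post-process volume and fires some-started or all-stopped notifications on changes.
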(event Custom|Recording%20Started
  ;[0.059 0.4375 0] Change count of recording actors, work out screen effect
  (Math|Integer|IncrementInt (Variables|Default|GetRewindingActors)
    (:%20%20
      (CallFunction|CalculateRewindEffect))))

(event Custom|Recording%20Stopped
  ;[0.059 0.4375 0] Change count of recording actors, work out screen effect
  (bind _result (Math|Integer|DecrementInt (Variables|Default|GetRewindingActors))
    (:%20%20
      ;;[0.059 0.4375 0] Stops it getting out of sync if somehow called multiples times (shouldn't be needed, but safer to have)
      (Variables|Default|SetRewindingActors (Math|Integer|Max(Integer) _result))
      (CallFunction|CalculateRewindEffect))))

(event EventBeginPlay
  (Utilities|FlowControl|Delay 0.2)
  ;[0.059 0.4375 0] Bind to stopped and started rewind events for all time reversing components. Keeps track of how many things are currently reversing
  (bind _outactors (Actor|GetAllActorswithTag "Time"))
  (for _array_element _outactors
    (for _array_element_2 (Actor|GetComponentsByClass _array_element "/TimeManipulation/Components/BP_TimeReverse.BP_TimeReverse_C")
      (EventDispatchers|BindEventtoStartingRewinding _array_element_2 (delegate Custom|Recording%20Started))
      (EventDispatchers|BindEventtoStoppedRewinding _array_element_2 (delegate Custom|Recording%20Stopped)))))

(fn ConstructionScript)

(fn StopRewind
  (params (Tag :type Name))
  ;[0.059 0.4375 0] Gets all actors with a tag matching the passed in tag
  (bind _outactors (Actor|GetAllActorswithTag Tag))
  (for _array_element _outactors
    ;[0.059 0.4375 0] Stops actors with that tag rewinding
    (for _array_element_2 (Actor|GetComponentsByClass _array_element "/TimeManipulation/Components/BP_TimeReverse.BP_TimeReverse_C")
      (bind _asbp_time_reverse (Utilities|Casting|CastToBP_TimeReverse _array_element_2))
      (Default|StopRewind _asbp_time_reverse))))

(fn StartRewind
  (params (Tag :type Name) (Speed :type Float%20%28double-precision%29))
  ;[0.059 0.4375 0] find all actors with the passed in tag
  (bind _outactors (Actor|GetAllActorswithTag Tag))
  (for _array_element _outactors
    ;[0.059 0.4375 0] Starts the actors with that tag rewinding
    (for _array_element_2 (Actor|GetComponentsByClass _array_element "/TimeManipulation/Components/BP_TimeReverse.BP_TimeReverse_C")
      (bind _asbp_time_reverse (Utilities|Casting|CastToBP_TimeReverse _array_element_2))
      (Default|StartRewind _asbp_time_reverse Speed))))

(fn StartRewindEffect
  (bind _postprocessvol (Variables|Default|GetPostProcessVol))
  ;[0.059 0.4375 0] Adds and starts the effect on the postprocessing volume, makes it infinite size
  (Utilities|IsValid _postprocessvol
    (:Is%20Valid
      (Variables|/Script/Engine.PostProcessVolume|SetSettings _postprocessvol (Utilities|Struct|MakePostProcessSettings (Utilities|Struct|MakeWeightedBlendables (Utilities|Array|MakeArray (Utilities|Struct|MakeWeightedBlendable 1.0 (Variables|Default|GetEffectMaterial))))))
      (Variables|/Script/Engine.PostProcessVolume|SetbUnbound _postprocessvol true))))

(fn StopRewindEffect
  (bind _postprocessvol (Variables|Default|GetPostProcessVol))
  ;[0.059 0.4375 0] Removes the effect from the post processing volume, stops it being infinite size
  (Utilities|IsValid _postprocessvol
    (:Is%20Valid
      (Variables|/Script/Engine.PostProcessVolume|SetSettings _postprocessvol (Utilities|Struct|MakePostProcessSettings (Utilities|Struct|MakeWeightedBlendables (Utilities|Array|MakeArray ""))))
      (Variables|/Script/Engine.PostProcessVolume|SetbUnbound _postprocessvol false))))

(fn GetIsReversing
  ;[0.059 0.4375 0] Whether or not the time manager is reversing
  (return (> (Variables|Default|GetRewindingActors) 0)))

(fn CalculateRewindEffect
  ;[0.059 0.4375 0] Work out whether or not the reverse effect needs to be added to the screen, if so, add it.
  (bind _reversing (CallFunction|GetIsReversing))
  (if _reversing
    (CallFunction|StartRewindEffect)
    (Default|CallSomeStartedRewinding)
    (else
      (CallFunction|StopRewindEffect)
      (Default|CallAllStoppedRewinding))))