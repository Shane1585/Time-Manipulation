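; BP_Highlight is an actor component that highlights its owning StaticMeshActor with an overlay material.
; When UseDistance is on, Tick (0.25 seconds by default) compares the player character's distance to HighlightRadius and calls HighlightObject or UnhighlightObject.
; These functions set or clear HighlightMaterial on the mesh, using IsHighlighted to skip redundant changes.
; A disconnected custom depth node never runs.
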(event EventTick
  (params (DeltaSeconds :type Float%20%28single-precision%29))
  ;[0.059 0.4375 0] Tick runs every 0.25 seconds by default here
  (if (Variables|Default|GetUseDistance)
    (if (<= (Transformation|GetDistanceTo (Game|GetPlayerCharacter 0) (Components|GetOwner)) (Variables|Default|GetHighlightRadius))
      (CallFunction|HighlightObject)
      (else
        (CallFunction|UnhighlightObject)))))

(fn HighlightObject
  ;[0.059 0.4375 0] Checks if the object is already highlighted, before trying to highlight it
  (if (not (Variables|Default|GetIsHighlighted?))
    ;[0.059 0.4375 0] Add the highlight material to the owning actor
    (bind _asstatic_mesh_actor (Utilities|Casting|CastToStaticMeshActor (Components|GetOwner)))
    (Rendering|Material|SetOverlayMaterial (Variables|/Script/Engine.StaticMeshActor|GetStaticMeshComponent _asstatic_mesh_actor) (Variables|Default|GetHighlightMaterial) :!class /Script/Engine.MeshComponent)
    ;[0.059 0.4375 0] flag as being highlighted
    (Variables|Default|SetIsHighlighted? true)))

(fn UnhighlightObject
  ;[0.059 0.4375 0] Checks if the object is  highlighted, before trying to unhighlight it
  (if (Variables|Default|GetIsHighlighted?)
    ;[0.059 0.4375 0] Remove the highlight material from owning actor
    (bind _asstatic_mesh_actor (Utilities|Casting|CastToStaticMeshActor (Components|GetOwner)))
    (Rendering|Material|SetOverlayMaterial (Variables|/Script/Engine.StaticMeshActor|GetStaticMeshComponent _asstatic_mesh_actor) 0 :!class /Script/Engine.MeshComponent)
    ;[0.059 0.4375 0] Flag as not highlighted
    (Variables|Default|SetIsHighlighted? false)))