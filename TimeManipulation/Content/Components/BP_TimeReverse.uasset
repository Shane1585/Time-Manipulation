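; BP_TimeReverse is an actor component that records its owner's movement and rewinds it at a chosen speed.
; Each tick it stores delta time, transform and mesh velocities, merging motionless frames up to a time cap.
; Rewinding disables physics and consumes frames backwards with transform lerps, restoring velocities and recording upon reaching the first frame.
; It tags owners as character or object time actors and can play a reverse montage on Characters.
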(event EventBeginPlay
  ;[1 1 1] sets the first frame in the array
  (|Setsuptags
    (:exec
      (if (Variables|Default|GetStartsOffRecording)
        (CallFunction|StartNewRecording)))))

(event EventTick
  (params (DeltaSeconds :type Float%20%28single-precision%29))
  ;[1 1 1] If "its recording" is true it will store every frame untill the point where is reversing is true
  (if (Variables|Default|GetIsRecording?)
    (CallFunction|StoresNextFrame DeltaSeconds)
    (else
      ;[1 1 1] if is recording is false the it checks if it is reversing if so its going to play back tthe frames in revers for the rewind of the plater of objects
      (if (Variables|Default|GetIsReversing?)
        (CallFunction|PlayBackFrames DeltaSeconds)))))

(fn StartNewRecording
  ;[0.059 0.4375 0] Wipes Frames array and sets first frame, stops it reversing, starts it recording
  (if (Variables|Default|GetIsReversing?)
    (Default|CallStoppedRewinding)
    (CallFunction|StopRewindAnimation))
  (bind _velocity (CallFunction|GetLinearVelocity))
  (bind _velocity_2 (CallFunction|GetAngularVelocity))
  (Variables|Default|SetFrames (Utilities|Array|MakeArray (Utilities|Struct|MakeST_FrameData 0.0 (Transformation|GetActorTransform (Components|GetOwner)) _velocity _velocity_2)))
  (Variables|Default|SetIsReversing? false)
  (Variables|Default|SetIsRecording? true))

(fn StoresNextFrame
  (params (DeltaTime :type Float%20%28double-precision%29))
  ;[0.059 0.4375 0] Creates the next frame or adds to the last frame if not moved, up to a cap of delta time in 'MaxTimeRecordingWhenStopped'
  (bind _velocity (CallFunction|GetAngularVelocity))
  (bind _velocity_2 (CallFunction|GetLinearVelocity))
  (bind _returnvalue (CallFunction|AreThereTwoFramesinFrames))
  (if _returnvalue
    (bind _hasntmoved (CallFunction|HasntMovedinLastTwoFrames))
    (if _hasntmoved
      (CallFunction|AddTimetoLastFrame DeltaTime)
      (else
        (Utilities|Array|Add (Variables|Default|GetFrames) (Utilities|Struct|MakeST_FrameData DeltaTime (Transformation|GetActorTransform (Components|GetOwner)) _velocity_2 _velocity) :!label _label)))
    (else
      (goto _label))))

(fn PlayBackFrames
  (params (DeltaTime :type Float%20%28double-precision%29))
  ;[0.059 0.4375 0] This is where all of the details about the Frames, DeltaTime along with the Velocity, Position and Location is used to reverse an actor the passed in amount of time
  (|SetStartingDetails (* DeltaTime (Variables|Default|GetReverseSpeed)) 0.0) ; Sets initial information about the actor (velocity, transform)
  (bind _index (Utilities|FlowControl|ForLoopwithBreak 0 (- (Utilities|Array|Length (Variables|Default|GetFrames)) 1) :!label _label) ; Loops until last frame, unless stopped
    (:LoopBody
      (|CalculateIfPassedLastFrame _index) ; Checks to see if we've gone past the last frame with the remaining amount of delta time to reverse, and into the frame before that
      (if (LocalVariables|GetPassedTheFrame?)
        ;;[0.059 0.4375 0] Removes the last frame, takes away its delta time from the time that's being reversed
        (|RemoveLastFrameAndTakeawayDaltaTme)
        (else
          (|MoveToLocationBasedOnLastFrame) ; Lerps between current location and last stored frame
          (|CountDownTheTimer) ; Decreases time left to reverse for the last frame
          (goto _label Break))))
    (:Completed
      ;;[0.059 0.4375 0] When reached the starting location (start of record), stop reversing and set starting velocity
      (if (Utilities|Array|IsEmpty (Variables|Default|GetFrames))
        (|Movetofinallocation)
        (Variables|Default|SetIsReversing? false)
        (Variables|Default|SetIsRecording? true)
        (CallFunction|StopRewindAnimation)
        (Default|CallStoppedRewinding)))))

(fn DebugLogDetails
  (params (text :type String))
  (bind _returnvalue (Math|DateTime|Now))
  ;[0.059 0.4375 0] A function used to debug
  (Development|PrintString (Utilities|String|Append text (Utilities|String|ToString(Transform) (Transformation|GetActorTransform (Components|GetOwner)))))
  (Development|PrintString (Utilities|String|Append (Utilities|String|ToString(Integer) (Class|KismetMathLibrary|GetHour _returnvalue)) ":" (Utilities|String|ToString(Integer) (Class|KismetMathLibrary|GetMinute _returnvalue)) ":" (Utilities|String|ToString(Integer) (Class|KismetMathLibrary|GetSecond _returnvalue)) ":" (Utilities|String|ToString(Integer) (Math|DateTime|GetMillisecond _returnvalue)))))

(fn GetLinearVelocity
  ;[0.059 0.4375 0] Gets linear velocity of the owner
  (bind _returnvalue (Physics|GetPhysicsLinearVelocity (Actor|GetComponentbyClass (Components|GetOwner) "/Script/Engine.StaticMeshComponent") "None"))
  (return _returnvalue))

(fn GetAngularVelocity
  ;[0.059 0.4375 0] Gets the angular velocity of the owner
  (return (Physics|GetPhysicsAngularVelocityinDegrees (Actor|GetComponentbyClass (Components|GetOwner) "/Script/Engine.StaticMeshComponent") "None")))

(fn SetLinearVelocity
  (params (Velocity :type Vector))
  ;[0.059 0.4375 0] Sets linear velocity of the owner to passed in velocity
  (Physics|SetPhysicsLinearVelocity (Actor|GetComponentbyClass (Components|GetOwner) "/Script/Engine.StaticMeshComponent") Velocity false "None")
  (return))

(fn SetAngularVelocity
  (params (Velocity :type Vector))
  ;[0.059 0.4375 0] Sets angular velocity of the owner to passed in velocity
  (Class|PrimitiveComponent|SetPhysicsAngularVelocityinDegrees (Actor|GetComponentbyClass (Components|GetOwner) "/Script/Engine.StaticMeshComponent") Velocity false "None")
  (return))

(fn StartRewind
  (params (Speed :type Float%20%28double-precision%29))
  ;[0.059 0.4375 0] At the start of the rewind it checks to see if there is more the two frames to rewind (if not the rewind and animation wont play)
  (Variables|Default|SetReverseSpeed Speed)
  (bind _returnvalue (CallFunction|AreThereTwoFramesinFrames))
  (if _returnvalue
    ;[0.059 0.4375 0] Play the chosen animation and set is reversing to true (so the reverse  will not be recorded)
    (CallFunction|PlayRewindAnimation)
    (Variables|Default|SetIsRecording? false)
    (Variables|Default|SetIsReversing? true)
    ;[0.059 0.4375 0] Remove Physics from the object - stop gravity and velocity from having an effect.
    (CallFunction|TurnOffPhysics)
    (CallFunction|SetLinearVelocity "0, 0, 0")
    (CallFunction|SetAngularVelocity "0, 0, 0")
    (Default|CallStartingRewinding)
    (return true)
    (else
      (return false))))

(fn TurnOffPhysics
  ;[0.059 0.4375 0] Turns off physics of owning actor
  (Physics|SetSimulatePhysics (Actor|GetComponentbyClass (Components|GetOwner) "/Script/Engine.StaticMeshComponent") false)
  (return))

(fn TurnonPhysics
  ;[0.059 0.4375 0] Turns on the physics of the owning actor
  (Physics|SetSimulatePhysics (Actor|GetComponentbyClass (Components|GetOwner) "/Script/Engine.StaticMeshComponent") true)
  (return))

(fn AreThereTwoFramesinFrames
  ;[0.059 0.4375 0] Checks if there are two or more stored frames in the array
  (return (>= (Utilities|Array|Length (Variables|Default|GetFrames)) 2)))

(fn DoesActorTransformMatchFrame
  (params (Number%20Of%20Frames%20From%20End :type Integer))
  (bind _frames (Variables|Default|GetFrames))
  ;[0.059 0.4375 0] Checks if the frame however many passed in from the end matches the current transform of the actor
  (return (== (.transform (Utilities|Array|Get(acopy) _frames (- (Utilities|Array|Length _frames) (+ Number%20Of%20Frames%20From%20End 1)))) (Transformation|GetActorTransform (Components|GetOwner)))))

(fn DoesActorLinVelocityMatchFrame
  (params (Number%20Of%20Frames%20From%20End :type Integer))
  (bind _frames (Variables|Default|GetFrames))
  ;[0.059 0.4375 0] Checks if the frame however many passed in from the end matches the current Linear velocity of the actor
  (bind _velocity (CallFunction|GetLinearVelocity))
  (return (Utilities|Operators|EqualEqual _velocity (.linearvelocity (Utilities|Array|Get(acopy) _frames (- (Utilities|Array|Length _frames) (+ Number%20Of%20Frames%20From%20End 1)))) 0.0)))

(fn DoesActorAngVelocityMatchFrame
  (params (Number%20Of%20Frames%20From%20End :type Integer))
  (bind _frames (Variables|Default|GetFrames))
  ;[0.059 0.4375 0] Checks if the frame however many passed in from the end matches the current angular velocity of the actor
  (bind _velocity (CallFunction|GetAngularVelocity))
  (return (Utilities|Operators|EqualEqual _velocity (.angularvelocity (Utilities|Array|Get(acopy) _frames (- (Utilities|Array|Length _frames) (+ Number%20Of%20Frames%20From%20End 1)))) 0.0)))

(fn AddTimetoLastFrame
  (params (Delta%20Time :type Float%20%28double-precision%29))
  (bind _frames (Variables|Default|GetFrames))
  (bind _returnvalue (Utilities|Array|Length _frames))
  (bind _returnvalue_2 (- _returnvalue 1))
  (bind _output (Utilities|Array|Get(acopy) _frames _returnvalue_2))
  ;[0.059 0.4375 0] Adds time to the last frame increasing what it previously was (this means it spent longer in same position and velocity)
  (|SetBy-RefVar (Utilities|Array|Get(acopy) _frames _returnvalue_2) (Utilities|Struct|MakeST_FrameData (Math|Float|Min(Float) (+ Delta%20Time (.deltatime _output)) (Variables|Default|GetMaxTimeRecordingWhenStopped)) (.transform _output) (.linearvelocity _output) (.angularvelocity _output))))

(fn HasntMovedinLastTwoFrames
  ;[0.059 0.4375 0] Check transform and velocities of the last two stored frames in the array match the current transform/velocity (meaning the actor hasn't moved)
  (bind _returnvalue (CallFunction|DoesActorTransformMatchFrame))
  (bind _returnvalue_2 (CallFunction|DoesActorLinVelocityMatchFrame))
  (bind _returnvalue_3 (CallFunction|DoesActorAngVelocityMatchFrame))
  (bind _returnvalue_4 (CallFunction|DoesActorTransformMatchFrame 1))
  (bind _returnvalue_5 (CallFunction|DoesActorLinVelocityMatchFrame 1))
  (bind _returnvalue_6 (CallFunction|DoesActorAngVelocityMatchFrame 1))
  (return (Math|Boolean|ANDBoolean _returnvalue _returnvalue_2 _returnvalue_3 _returnvalue_4 _returnvalue_5 _returnvalue_6)))

(fn StopRewind
  ;[0.059 0.4375 0] When the rewind is stopped it enables physics and stops the animation on the actor effected.
  (Variables|Default|SetIsReversing? false)
  (CallFunction|TurnonPhysics)
  (CallFunction|StopRewindAnimation)
  (Default|CallStoppedRewinding)
  (return))

(fn StopRecording
  ;[0.059 0.4375 0] Stops the recording everything about the actor (not rewinding)
  (Variables|Default|SetFrames (Utilities|Array|MakeArray ""))
  (Variables|Default|SetIsReversing? false)
  (Variables|Default|SetIsRecording? false))

(fn PlayRewindAnimation
  ;[0.059 0.4375 0] Uses default falling animation when reversing the player (only reverses if plays reverse animation is true in component)
  (if (Variables|Default|GetPlaysReverseAnimation)
    (bind _ascharacter (Utilities|Casting|CastToCharacter (Components|GetOwner)))
    (Animation|PlayAnimMontage _ascharacter (Variables|Default|GetReverseMontage) (* (Variables|Default|GetReverseSpeed) 1.5) "None")))

(fn StopRewindAnimation
  ;[0.059 0.4375 0] Uses default falling animation when reversing the player (only reverses if plays reverse animation is true in component)
  (if (Variables|Default|GetPlaysReverseAnimation)
    (bind _ascharacter (Utilities|Casting|CastToCharacter (Components|GetOwner)))
    (Animation|StopAnimMontage _ascharacter (Animation|GetCurrentMontage _ascharacter :!class /Script/Engine.Character))))